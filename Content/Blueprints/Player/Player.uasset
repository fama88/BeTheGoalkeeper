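; Player pawn that the mouse moves in the world Y-Z plane.
; MouseX and MouseY axis values are clamped to unit range, scaled by SpeedMovement and fed to AddMovementInput along world Y and Z respectively.
; Tick and the construction script are empty, and a Velocity times DeltaSeconds calculation is left unused.
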(event `InputAxis|MouseX`
  (params (AxisValue :type "Float (single-precision)"))
  ;[1 1 1] Mouse Left/Right Event
  (`self.AddMovementInput` (0.0 1.0 0.0) (* (`KismetMathLibrary.FClamp` AxisValue -1.0) (`self.SpeedMovement`))))

(event `InputAxis|MouseY`
  (params (AxisValue :type "Float (single-precision)"))
  ;[1 1 1] Mouse Up/Down Event
  (`self.AddMovementInput` (0.0 0.0 1.0) (* (`KismetMathLibrary.FClamp` AxisValue -1.0) (`self.SpeedMovement`))))

(event `self.ReceiveTick`
  (params (DeltaSeconds :type "Float (single-precision)")))

(fn `UserConstructionScript`)