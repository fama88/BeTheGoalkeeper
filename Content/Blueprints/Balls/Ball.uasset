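; Ball actor that launches itself in a randomized direction when play begins and can be reset to its starting spot.
; HitBallInRandomDirection enables physics, saves the initial transform, then applies an impulse along the forward vector with random pitch and yaw offsets, scaled by ImpulseForce.
; RelocateBall restores the saved transform, disables physics and prints a debug string, but is not called within this Blueprint.
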(event `self.ReceiveBeginPlay`
  (`self.HitBallInRandomDirection`))

(fn `HitBallInRandomDirection`
  (`PrimitiveComponent.SetSimulatePhysics` (`self.Ball`) true)
  (set `self.InitWorldRotation` (`self.K2_GetActorRotation`))
  (set `self.InitWorldLocation` (`self.K2_GetActorLocation`))
  (`PrimitiveComponent.AddImpulse` (`self.Ball`) (* (`KismetMathLibrary.Conv_RotatorToVector` (`KismetMathLibrary.MakeRotator` (.roll (`KismetMathLibrary.Conv_VectorToRotator` (`SceneComponent.GetForwardVector` (`self.Ball`)))) (+ (.pitch (`KismetMathLibrary.Conv_VectorToRotator` (`SceneComponent.GetForwardVector` (`self.Ball`)))) (* (`KismetMathLibrary.RandomFloat`) (`self.Roll Max`))) (+ (.yaw (`KismetMathLibrary.Conv_VectorToRotator` (`SceneComponent.GetForwardVector` (`self.Ball`)))) (`KismetMathLibrary.RandomFloatInRange` (`self.YawMin`) (`self.Yaw Max`))))) (`self.ImpulseForce`)) "None" false))

(fn `RelocateBall`
  (`KismetSystemLibrary.PrintString` "RelocateCalled")
  (`self.K2_SetActorLocationAndRotation` (`self.InitWorldLocation`) (`self.InitWorldRotation`))
  (`PrimitiveComponent.SetSimulatePhysics` (`self.Ball`) false))

(fn `UserConstructionScript`)